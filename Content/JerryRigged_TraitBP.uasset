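; Jerry-Rigged mech trait that boosts structure health on chosen parts and scales down refit costs.
; ApplyTrait gathers health components from ApplicableMechParts and adds IncreasedStructurePercent to each one's trait multiplier.
; The same loop rewrites the RefitCosts data asset itself, so the ReducedRefitCostsPercent scaling compounds per component, and right-leg replace time is multiplied by zero.
; UI functions report per-part bonus and description values.
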(fn `ApplyTrait`
  (params (InMech :type "MWMech Object Reference"))
  (locals (`Increase Health Multiplier` :type "Float (double-precision)" :default 0.0))
  (bind _reduced_refit_costs_percent (`self.Reduced Refit Costs Percent`))
  (bind _returnvalue (`MWMechRefitCostsDataAsset.GetAsset` (`.RefitCosts` (break `MechData` (`MWMechDataAsset.MechData` (`MWMech.GetMechDataAsset` InMech))))))
  (bind (_head_replacebasecbillcost _centertorso_replacebasecbillcost _lefttorso_replacebasecbillcost _righttorso_replacebasecbillcost _leftarm_replacebasecbillcost _rightarm_replacebasecbillcost _leftleg_replacebasecbillcost _rightleg_replacebasecbillcost _head_partreplacetimecost _centertorso_partreplacetimecost _lefttorso_partreplacetimecost _righttorso_partreplacetimecost _leftarm_partreplacetimecost _rightarm_partreplacetimecost _leftleg_partreplacetimecost _rightleg_partreplacetimecost) (break `MechRefitCosts` (`MWMechRefitCostsDataAsset.RefitCosts` _returnvalue)))
  (bind _outhealthcomponent (`self.GetHealthComponents` InMech))
  (for _array_element _outhealthcomponent
    (`self.Helper_BoostHealthComponent` _array_element)
    (set `MWMechRefitCostsDataAsset.RefitCosts` (make `MechRefitCosts` (`KismetMathLibrary.FTrunc` (* _head_replacebasecbillcost _reduced_refit_costs_percent)) (`KismetMathLibrary.FTrunc` (* _centertorso_replacebasecbillcost _reduced_refit_costs_percent)) (`KismetMathLibrary.FTrunc` (* _lefttorso_replacebasecbillcost _reduced_refit_costs_percent)) (`KismetMathLibrary.FTrunc` (* _righttorso_replacebasecbillcost _reduced_refit_costs_percent)) (`KismetMathLibrary.FTrunc` (* _leftarm_replacebasecbillcost _reduced_refit_costs_percent)) (`KismetMathLibrary.FTrunc` (* _rightarm_replacebasecbillcost _reduced_refit_costs_percent)) (`KismetMathLibrary.FTrunc` (* _leftleg_replacebasecbillcost _reduced_refit_costs_percent)) (`KismetMathLibrary.FTrunc` (* _rightleg_replacebasecbillcost _reduced_refit_costs_percent)) (* _head_partreplacetimecost _reduced_refit_costs_percent) (* _centertorso_partreplacetimecost _reduced_refit_costs_percent) (* _lefttorso_partreplacetimecost _reduced_refit_costs_percent) (* _righttorso_partreplacetimecost _reduced_refit_costs_percent) (* _leftarm_partreplacetimecost _reduced_refit_costs_percent) (* _rightarm_partreplacetimecost _reduced_refit_costs_percent) (* _leftleg_partreplacetimecost _reduced_refit_costs_percent) (* _rightleg_partreplacetimecost 0.0)) _returnvalue)))

(fn `GetHealthComponents`
  (params (InMech :type "MWMech Object Reference"))
  (returns (OutHealthComponent :type "Array of MWHealthComponent Object Reference"))
  (locals (L_HealthComponents :type "Array of MWHealthComponent Object Reference"))
  (bind _l_healthcomponents (`local.L_HealthComponents`))
  (bind _mechlivingactorcomponent (`MWMech.MechLivingActorComponent` (`local.InMech`)))
  (for _array_element (`self.ApplicableMechParts`)
    (switch `EMechParts` _array_element
      (:`Head`
        (`KismetArrayLibrary.Array_AddUnique` _l_healthcomponents (`MWMechLivingActorComponent.Head` _mechlivingactorcomponent)))
      (:`CenterTorso`
        (`KismetArrayLibrary.Array_AddUnique` _l_healthcomponents (`MWMechLivingActorComponent.CenterTorso` _mechlivingactorcomponent)))
      (:`LeftTorso`
        (`KismetArrayLibrary.Array_AddUnique` _l_healthcomponents (`MWMechLivingActorComponent.LeftTorso` _mechlivingactorcomponent)))
      (:`LeftArm`
        (`KismetArrayLibrary.Array_AddUnique` _l_healthcomponents (`MWMechLivingActorComponent.LeftArm` _mechlivingactorcomponent)))
      (:`LeftLeg`
        (`KismetArrayLibrary.Array_AddUnique` _l_healthcomponents (`MWMechLivingActorComponent.LeftLeg` _mechlivingactorcomponent)))
      (:`RightTorso`
        (`KismetArrayLibrary.Array_AddUnique` _l_healthcomponents (`MWMechLivingActorComponent.RightTorso` _mechlivingactorcomponent)))
      (:`RightArm`
        (`KismetArrayLibrary.Array_AddUnique` _l_healthcomponents (`MWMechLivingActorComponent.RightArm` _mechlivingactorcomponent)))
      (:`RightLeg`
        (`KismetArrayLibrary.Array_AddUnique` _l_healthcomponents (`MWMechLivingActorComponent.RightLeg` _mechlivingactorcomponent)))))
  (return (`local.L_HealthComponents`)))

(fn `Helper_BoostHealthComponent`
  (params (`In Health Component` :type "MWHealthComponent Object Reference"))
  (`MWHealthComponent.SetHealthTraitMultiplierPercent` `In Health Component` (+ (`self.Increased Structure Percent`) (`MWHealthComponent.HealthTraitMultiplierPercent` `In Health Component`))))

(fn `UI_GetDisplayArguments`
  (returns (ReturnValue :type "Array of NamedArgumentPair Structure"))
  (return (`|MakeArray` (make `NamedArgumentPair` "0" (`KismetTextLibrary.Conv_TextToString` (`KismetTextLibrary.Conv_DoubleToText` (* (`self.Increased Structure Percent`) 100.0) "HalfToEven" true true 1 324 0 2))) (make `NamedArgumentPair` "1" (`KismetTextLibrary.Conv_TextToString` (`KismetTextLibrary.Conv_DoubleToText` (`self.Display Percent`) "HalfToEven" true true 1 324 0 2))))))

(fn `UI_GetIncreasedStructurePercent`
  (params (MechPart :type "EMechParts Enum" :default "Head"))
  (returns (ReturnValue :type "Float (double-precision)"))
  (if (`KismetArrayLibrary.Array_Contains` (`self.ApplicableMechParts`) MechPart)
    (return (`self.Increased Structure Percent`))
    (else
      (return 0.0))))